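; BP_Wizard is a wizard character Blueprint that handles player locomotion through Enhanced Input.
; On BeginPlay it casts and stores the BP_PlayerController, then adds the IMC_Locomotion mapping context to that controller's input subsystem.
; The IA_Move action drives movement input along right and forward vectors derived from control rotation, so movement follows the camera's yaw.
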(event Input|EnhancedActionEvents|EnhancedInputActionIA_Move
  (params (ActionValue :type Vector%202D%20Structure) (ElapsedSeconds :type Float%20%28double-precision%29) (TriggeredSeconds :type Float%20%28double-precision%29) (InputAction :type Input%20Action%20Object%20Reference :default "/Game/Inputs/Actions/IA_Move.IA_Move"))
  (bind _returnvalue (Pawn|GetControlRotation :!class /Script/Engine.Pawn))
  ;[0.02843 0.2159 0.8469] Movement
  (Pawn|Input|AddMovementInput (Math|Vector|GetRightVector (Math|Rotator|MakeRotator (.roll _returnvalue) 0.0 (.yaw _returnvalue))) (.x ActionValue) false)
  (Pawn|Input|AddMovementInput (Math|Vector|GetForwardVector (Math|Rotator|MakeRotator 0.0 0.0 (.yaw (Pawn|GetControlRotation :!class /Script/Engine.Pawn)))) (.y ActionValue) false))

(event EventBeginPlay
  (bind _asbp_player_controller (Utilities|Casting|CastToBP_PlayerController (Game|GetPlayerController 0)))
  (bind _output_get (Variables|Default|SetPlayerControllerRef _asbp_player_controller))
  (Input|AddMappingContext (PlayerController|LocalPlayerSubsystems|GetEnhancedInputLocalPlayerSubsystem _output_get) "/Game/Inputs/IMC_Locomotion.IMC_Locomotion" 0 "(bIgnoreAllPressedKeysUntilRelease=True,bForceImmediately=False,bNotifyUserSettings=False)"))

(event Collision|EventActorBeginOverlap
  (params (OtherActor :type Actor%20Object%20Reference)))

(event EventTick
  (params (DeltaSeconds :type Float%20%28single-precision%29)))

(fn ConstructionScript)